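; Goal_BP is a goal zone that destroys any Ball entering it and awards a point to the opposing player.
; On BeginPlay it casts player 0's pawn to Paddle_BP and caches it as a reference.
; When its Box overlaps a Ball, the Player1Goal flag selects whether Player 2's or Player 1's score updates through that paddle's ScoreHub.
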(event OnComponentBeginOverlap(Box)
  (params (OverlappedComponent :type Primitive%20Component%20Object%20Reference) (OtherActor :type Actor%20Object%20Reference) (OtherComp :type Primitive%20Component%20Object%20Reference) (OtherBodyIndex :type Integer) (bFromSweep :type Boolean) (SweepResult :type Hit%20Result%20Structure%20%28by%20ref%29))
  (bind _asball (Utilities|Casting|CastToBall OtherActor))
  (Actor|DestroyActor _asball)
  (if (Variables|Default|GetPlayer1Goal?)
    (Default|UpdatePlayer2Score (Variables|/Game/Blueprints/Paddle_BP.Paddle_BP_C|GetScoreHub (Variables|Default|GetPaddleReference)))
    (else
      (Default|UpdatePlayer1Score (Variables|/Game/Blueprints/Paddle_BP.Paddle_BP_C|GetScoreHub (Variables|Default|GetPaddleReference))))))

(event EventBeginPlay
  (bind _aspaddle_bp (Utilities|Casting|CastToPaddle_BP (Game|Player|GetPlayerPawn 0)))
  (Variables|Default|SetPaddleReference _aspaddle_bp))

(event Collision|EventActorBeginOverlap
  (params (OtherActor :type Actor%20Object%20Reference)))

(event EventTick
  (params (DeltaSeconds :type Float%20%28single-precision%29)))

(fn ConstructionScript)