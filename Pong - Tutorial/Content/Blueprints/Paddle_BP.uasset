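; Player paddle pawn for a Pong-style game, moved sideways through Enhanced Input.
; On BeginPlay it adds the Pinpong input mapping context to its player controller, then creates and shows the score widget, keeping a reference to it.
; The move action offsets the cube along local Y by the input value times player speed, with sweep so collisions block it.
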(event Input|EnhancedActionEvents|EnhancedInputActionMove_IA
  (params (ActionValue :type Float%20%28double-precision%29) (ElapsedSeconds :type Float%20%28double-precision%29) (TriggeredSeconds :type Float%20%28double-precision%29) (InputAction :type Input%20Action%20Object%20Reference :default "/Game/Input/Move_IA.Move_IA"))
  (Transformation|AddLocalOffset (Variables|Default|GetCube) (Math|Vector|MakeVector 0.0 (* ActionValue (Variables|Default|GetPlayerspeed)) 0.0) true false))

(event EventBeginPlay
  (bind _asplayer_controller (Utilities|Casting|CastToPlayerController (Pawn|GetController)))
  (Utilities|IsValid (PlayerController|LocalPlayerSubsystems|GetEnhancedInputLocalPlayerSubsystem _asplayer_controller)
    (:Is%20Valid
      (Input|AddMappingContext (PlayerController|LocalPlayerSubsystems|GetEnhancedInputLocalPlayerSubsystem _asplayer_controller) "/Game/Input/Pinpong_IMC.Pinpong_IMC" 0 "(bIgnoreAllPressedKeysUntilRelease=True,bForceImmediately=False,bNotifyUserSettings=False)")
      (bind _returnvalue (UserInterface|CreateWidget "/Game/Blueprints/Score_WB.Score_WB_C"))
      (bind _output_get (Variables|Default|SetScoreHub _returnvalue))
      (UserInterface|Viewport|AddtoViewport _output_get 0))))

(fn ConstructionScript)