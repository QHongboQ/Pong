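; Ball actor for a paddle game, driven by physics on its Sphere component.
; On BeginPlay it finds the Paddle_AI actor, hands it a reference to itself, and launches along negative X with a velocity-change impulse.
; Each hit raises BallSpeed by a fixed step and clamps the linear velocity to exactly that magnitude, so the ball keeps its direction and speeds up with every bounce.
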(event EventBeginPlay
  (bind _returnvalue (Actor|GetActorOfClass "/Game/Blueprints/Paddle_AI.Paddle_AI_C"))
  (bind _output_get (Variables|Default|SetAI%20REF _returnvalue))
  (Variables|/Game/Blueprints/Paddle_AI.Paddle_AI_C|SetBallReference _output_get self)
  (Physics|AddImpulse (Variables|Default|GetSphere) (Math|Vector|MakeVector -1e+03 0.0 0.0) "None" true))

(event Collision|EventActorBeginOverlap
  (params (OtherActor :type Actor%20Object%20Reference)))

(event EventTick
  (params (DeltaSeconds :type Float%20%28single-precision%29)))

(event Collision|EventHit
  (params (MyComp :type Primitive%20Component%20Object%20Reference) (Other :type Actor%20Object%20Reference) (OtherComp :type Primitive%20Component%20Object%20Reference) (bSelfMoved :type Boolean) (HitLocation :type Vector :default "0, 0, 0") (HitNormal :type Vector :default "0, 0, 0") (NormalImpulse :type Vector :default "0, 0, 0") (Hit :type Hit%20Result%20Structure%20%28by%20ref%29))
  (bind _sphere (Variables|Default|GetSphere))
  (Variables|Default|SetBallSpeed (+ (Variables|Default|GetBallSpeed) 15.0))
  (bind _returnvalue (Physics|GetPhysicsLinearVelocity _sphere "None"))
  (Physics|SetPhysicsLinearVelocity _sphere (Math|Vector|ClampVectorSize _returnvalue (Variables|Default|GetBallSpeed) (Variables|Default|GetBallSpeed)) false "None")
  (Physics|GetPhysicsLinearVelocity (Variables|Default|GetSphere) "None"))

(fn ConstructionScript)